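; Buggy vehicle Blueprint that acts as the win trigger when a ThirdPersonCharacter overlaps its collision.
; The win requires the character to have the key and a Fuel value of exactly zero.
; It then stops and disables character movement and plays a one-shot Macarena dance animation.
; After a fixed delay it pauses the game and shows the Winscreen widget.
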(event `self.Collision.OnComponentBeginOverlap`
  (params (OverlappedComponent :type "PrimitiveComponent Object Reference") (OtherActor :type "Actor Object Reference") (OtherComp :type "PrimitiveComponent Object Reference") (OtherBodyIndex :type Integer) (bFromSweep :type Boolean) (SweepResult :type "HitResult Structure (by ref)"))
  (bind _asthird_person_character (cast `/Game/ThirdPersonBP/Blueprints/ThirdPersonCharacter` OtherActor))
  (if (and (`/Game/ThirdPersonBP/Blueprints/ThirdPersonCharacter.HasKey` _asthird_person_character) (== (`/Game/ThirdPersonBP/Blueprints/ThirdPersonCharacter.Fuel` _asthird_person_character) 0))
    (`CharacterMovementComponent.DisableMovement` (`Character.CharacterMovement` _asthird_person_character))
    (`MovementComponent.StopMovementImmediately` (`Character.CharacterMovement` _asthird_person_character))
    (`SkeletalMeshComponent.PlayAnimation` (`Character.Mesh` _asthird_person_character) "/Game/Character/Animations/CricketBat/Macarena_Dance.Macarena_Dance" false)
    (`KismetSystemLibrary.Delay` 9.0)
    (`GameplayStatics.SetGamePaused` true)
    (bind _returnvalue (`|CreateWidget` "/Game/ThirdPersonBP/Blueprints/winscreen.winscreen_C"))
    (`UserWidget.AddToViewport` _returnvalue 0)))

(fn `UserConstructionScript`)